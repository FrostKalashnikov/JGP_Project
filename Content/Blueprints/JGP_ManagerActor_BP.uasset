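; Server-authoritative manager actor that runs timed photo-shot and recording sessions for users queued as JSON files.
; While idle, Tick polls a folder, reads user and quiz ID from the first file, fires OnStartExecution, then deletes it.
; Execution calls TakeShot, StartRecord and StopRecord dispatchers on fixed delays; its own handlers mostly print.
; Stopping starts a retriggerable cooldown before the next poll, which Enter clears early.
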(event `self.ReceiveBeginPlay`
  (`/Engine/EditorBlueprintResources/ActorMacros.Switch Has Authority`
    (:`Authority`
      (add `self.OnStartExecution` (`|CreateDelegate` :!event `OnStartExecution_Event`))
      (add `self.StartRecord` (`|CreateDelegate` :!event `StartRecord_Event`))
      (add `self.TakeShot` (`|CreateDelegate` :!event `TakeShot_Event`))
      (add `self.StopRecord` (`|CreateDelegate` :!event `StopRecord_Event`)))))

(event `StartRecord_Event`
  (`KismetSystemLibrary.PrintString` "Start Record"))

(event `TakeShot_Event`
  (`KismetSystemLibrary.PrintString` "Take Shot"))

(event `self.ReceiveTick`
  (params (DeltaSeconds :type "Float (single-precision)"))
  (`/Engine/EditorBlueprintResources/ActorMacros.Switch Has Authority`
    (:`Authority`
      (if (and (not (`self.InExecution`)) (not (`self.WaitingTime`)) true)
        (`self.CheckFile`)))))

(event `StopRecord_Event`
  (`KismetSystemLibrary.PrintString` "Stop Record")
  (set `self.InExecution` false)
  (`|ExecutionSequence`
    (:`then_0`
      (set `self.WaitingTime` true)
      (`KismetSystemLibrary.RetriggerableDelay` (`self.TimeDuration`))
      (set `self.WaitingTime` false))))

(event `OnStartExecution_Event` :!signature `self.OnStartExecution`
  (params (UserName :type String) (UserQuizID :type Integer))
  (set `self.InExecution` true)
  (set `self.CanCallNext` false)
  (`KismetSystemLibrary.Delay` 10.5)
  (`self.TakeShot`)
  (`KismetSystemLibrary.Delay` 3.0)
  (`self.StartRecord`)
  (`KismetSystemLibrary.Delay` 10.0)
  (`self.StopRecord`))

(event `Key|Enter`
  (params (Key :type "Key Structure"))
  (:`Pressed`
    (set `self.WaitingTime` false)
    (`KismetSystemLibrary.PrintString` "WAIT TIME OFF")))

(fn `CheckFile`
  (bind _filepath (`self.FilePath`))
  (bind (_foundfiles _returnvalue) (`BlueprintFileUtilsBPLibrary.FindFiles` _filepath ".json"))
  (if _returnvalue
    (bind _output (`|GetArrayItem` _foundfiles))
    (set `self.JsonPath` (`KismetStringLibrary.Concat_StrStr` _filepath "\\" _output))
    (`KismetSystemLibrary.PrintString` _output)
    (bind (_outjsonobject _returnvalue_2) (`JsonBlueprintFunctionLibrary.FromFile` (make `FilePath` (`self.JsonPath`))))
    (if _returnvalue_2
      (set `self.JsonFound` _outjsonobject)
      (bind (_outvalue _returnvalue_3) (`|GetJsonField` (`self.JsonFound`) "user"))
      (if _returnvalue_3
        (set `self.ReadedName` _outvalue)
        (bind (_outvalue_2 _returnvalue_4) (`|GetJsonField` (`self.JsonFound`) "userQuiz"))
        (if _returnvalue_4
          (set `self.QuizID` _outvalue_2)
          (`self.OnStartExecution` (`self.ReadedName`) (`self.QuizID`))
          (`BlueprintFileUtilsBPLibrary.DeleteFile` (`self.JsonPath`))
          (else
            (`KismetSystemLibrary.PrintString` "UserQuiz not found" true true (struct :`G` 1.0 :`A` 1.0))))
        (else
          (`KismetSystemLibrary.PrintString` "User not found" true true (struct :`G` 1.0 :`A` 1.0))))
      (else
        (`KismetSystemLibrary.PrintString` "File Not Found" true false (struct :`R` 1.0 :`A` 1.0) 0.4 :!label _label)))
    (else
      (goto _label))))

(fn `UserConstructionScript`)