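; ViewPawn_BP is a pawn Blueprint with debug keys for starting or joining a LAN multiplayer session.
; On BeginPlay or T, it runs the FPS and unit graph stat commands, sets Game and UI input and shows the mouse cursor.
; Key 1 creates a LAN session, then opens SceneCaptured as a listen server on success.
; Key 2 joins through an open command to a hard-coded IP address.
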(event `Key|T`
  (params (Key :type "Key Structure"))
  (bind _returnvalue (`GameplayStatics.GetPlayerController` 0))
  (:`Pressed`
    (`KismetSystemLibrary.ExecuteConsoleCommand` "stat unitgraph" null :!label _label)
    (`KismetSystemLibrary.ExecuteConsoleCommand` "stat fps" null)
    (`WidgetBlueprintLibrary.SetInputMode_GameAndUIEx` _returnvalue null)
    (set `PlayerController.bShowMouseCursor` true _returnvalue)))

(event `self.ReceiveBeginPlay`
  (goto _label))

(event `Key|One`
  (params (Key :type "Key Structure"))
  (:`Pressed`
    (`CreateSessionCallbackProxy.CreateSession` (`GameplayStatics.GetPlayerController` 0) 2 true
      (:`OnSuccess`
        (`KismetSystemLibrary.PrintString` "Success")
        (`GameplayStatics.OpenLevel` "SceneCaptured" true "listen"))
      (:`OnFailure`
        (`KismetSystemLibrary.PrintString` "Fail")))))

(event `Key|Two`
  (params (Key :type "Key Structure"))
  (:`Pressed`
    (`KismetSystemLibrary.ExecuteConsoleCommand` "open 192.168.18.221" null)
    (`KismetSystemLibrary.PrintString` "Openning")))

(fn `UserConstructionScript`)