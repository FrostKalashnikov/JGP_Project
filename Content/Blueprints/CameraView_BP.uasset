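; CameraView_BP is an actor that starts playback of a camera feed through the CameraMP media player.
; On BeginPlay it casts the game instance to GameInst, caches it and reads the CameraDevice stored there.
; It opens that device's URL on CameraMP and falls back to opening MediaSource if that call fails.
; Tick, overlap and construction logic are empty.
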(event `self.ReceiveBeginPlay`
  (bind _asgame_inst (cast `/Game/Blueprints/Base/GameInst` (`GameplayStatics.GetGameInstance`)))
  (bind _output_get (set `self.As Game Inst` _asgame_inst))
  (set `self.CameraDevice` (`/Game/Blueprints/Base/GameInst.Camera Device` _output_get))
  (bind _returnvalue (`MediaPlayer.OpenUrl` (`self.CameraMP`) (`.Url` (break `MediaCaptureDevice` (`self.CameraDevice`)))))
  (if (not _returnvalue)
    (`MediaPlayer.OpenSource` (`self.CameraMP`) (`self.Media Source`))))

(fn `UserConstructionScript`)