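; Child record-camera manager that captures video and screenshots on request from the JGP manager actor.
; On BeginPlay it finds JGP_ManagerActor_BP and binds to its start-record, stop-record and take-shot events, which start or finish capture or export the camera view texture as an "Original_" PNG.
; When an export finishes, it moves the file from the recording output directory to the content folder and prints the source path.
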(event `self.ReceiveBeginPlay`
  (bind _returnvalue (`GameplayStatics.GetActorOfClass` "/Game/Blueprints/JGP_ManagerActor_BP.JGP_ManagerActor_BP_C"))
  (bind _output_get (set `self.Manager` _returnvalue))
  (add `/Game/Blueprints/JGP_ManagerActor_BP.StartRecord` _output_get (`|CreateDelegate` :!event `Start Record`))
  (add `/Game/Blueprints/JGP_ManagerActor_BP.StopRecord` _output_get (`|CreateDelegate` :!event `Stop Record`))
  (add `/Game/Blueprints/JGP_ManagerActor_BP.TakeShot` _output_get (`|CreateDelegate` :!event `Take Shot`)))

(event `Start Record`
  (`self.StartCapture`))

(event `Stop Record`
  (`self.FinishCapture`))

(event `Take Shot`
  (`ImageWriteBlueprintLibrary.ExportToDisk` (`self.GetCameraViewTexture`) (`KismetStringLibrary.Concat_StrStr` (`self.ContentFolder`) "/" "Original_" (`self.GetFormattedFileName` false) ".png") (`self.ShotOptions`)))

(event `self.OnExportFinish`
  (bind _returnvalue (`self.GetFormattedFileName` true))
  (bind _returnvalue_2 (`KismetStringLibrary.Concat_StrStr` (`.Path` (break `DirectoryPath` (`.OutputDirectory` (break `RecordingSettings` (`self.RecordingSettings`))))) "/" _returnvalue))
  (`BlueprintFileUtilsBPLibrary.MoveFile` (`KismetStringLibrary.Concat_StrStr` (`self.ContentFolder`) "/" _returnvalue) _returnvalue_2)
  (`KismetSystemLibrary.PrintString` _returnvalue_2))

(fn `UserConstructionScript`
  (`parent.UserConstructionScript`))