(event `self.ReceiveBeginPlay`
  (`self.Set Text Rep` "")
  (bind _returnvalue (`GameplayStatics.GetActorOfClass` "/Game/Blueprints/JGP_ManagerActor_BP.JGP_ManagerActor_BP_C"))
  (bind _output_get (set `self.Manager` _returnvalue))
  (add `/Game/Blueprints/JGP_ManagerActor_BP.OnStartExecution` _output_get (`|CreateDelegate` :!event `Start`))
  (add `/Game/Blueprints/JGP_ManagerActor_BP.StartRecord` _output_get (`|CreateDelegate` :!event `Rec`))
  (add `/Game/Blueprints/JGP_ManagerActor_BP.StopRecord` _output_get (`|CreateDelegate` :!event `End`)))

(event `Set Text Rep`
  (params (TextValue :type Text))
  (set `self.TextValue` TextValue)
  (`TextRenderComponent.K2_SetText` (`self.TextRender`) (`self.TextValue`)))

(event `Start`
  (params (UserName :type String) (UserQuizID :type Integer))
  (`self.Set Text Rep` "Sorria para a foto"))

(event `Rec`
  (`self.Set Text Rep` "Prepare-se você está sendo filmado."))

(event `End`
  (`self.Set Text Rep` "dirigia-se e pegue a sua foto,  \nobrigado pela sua participação! \n"))

(fn `UserConstructionScript`)