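; LedPainel_BP is an LED panel actor that holds two planes and a camera rig with a spring arm.
; All logic runs in the Construction Script, which applies exposed values to the spring arm length and camera field of view.
; A shared distance value offsets PlaneA along local Y and PlaneB along negative local X.
; The event graph holds only disabled stubs, so the Blueprint adds no runtime behavior.
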(fn `UserConstructionScript`
  (set `SpringArmComponent.TargetArmLength` (`self.Target Arm Length`) (`self.SpringArm`))
  (`CameraComponent.SetFieldOfView` (`self.Camera`) (`self.In Field Of View`))
  (`SceneComponent.K2_SetRelativeLocation` (`self.PlaneA`) (`KismetMathLibrary.MakeVector` 0.0 (`self.Distance Painel`)) false false)
  (`SceneComponent.K2_SetRelativeLocation` (`self.PlaneB`) (`KismetMathLibrary.MakeVector` (* (`self.Distance Painel`) -1.0)) false false))